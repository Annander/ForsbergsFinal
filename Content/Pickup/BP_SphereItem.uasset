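; BP_SphereItem is a sphere pickup item that highlights when looked at and reports when picked up.
; The construction script creates a dynamic instance of M_PickupMaterial on the sphere and sets its Color to a default.
; LookEnter and LookExit events swap that Color parameter between enter and default colors, while Pickup only prints a debug message.
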(event `self.LookEnter`
  (`MaterialInstanceDynamic.SetVectorParameterValue` (`self.MaterialInstance`) "Color" (`self.EnterColor`)))

(event `self.LookExit`
  (`MaterialInstanceDynamic.SetVectorParameterValue` (`self.MaterialInstance`) "Color" (`self.DefaultColor`)))

(event `self.Pickup`
  (`KismetSystemLibrary.PrintString` "Picked up a thing!"))

(fn `UserConstructionScript`
  (bind _sphere (`self.Sphere`))
  (bind _returnvalue (`PrimitiveComponent.CreateDynamicMaterialInstance` _sphere 0 "/Game/Pickup/M_PickupMaterial.M_PickupMaterial" "None"))
  (bind _output_get (set `self.MaterialInstance` _returnvalue))
  (`PrimitiveComponent.SetMaterial` _sphere 0 _output_get)
  (`MaterialInstanceDynamic.SetVectorParameterValue` _output_get "Color" (`self.DefaultColor`)))