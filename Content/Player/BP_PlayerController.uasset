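; Player controller that routes Enhanced Input to the pawn it possesses.
; On possession it adds the input mapping context and stores the pawn, provided the local player's input subsystem is valid.
; Move, Look and Interact actions are forwarded to the stored pawn as messages, leaving the response to the pawn.
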(event `self.ReceivePossess`
  (params (PossessedPawn :type "Pawn Object Reference"))
  (bind _returnvalue (subsystem `EnhancedInputLocalPlayerSubsystem`))
  (`/Engine/EditorBlueprintResources/StandardMacros.IsValid` _returnvalue
    (:`Is Valid`
      (`EnhancedInputSubsystemInterface.AddMappingContext` _returnvalue "/Game/Player/IMC_InputMap.IMC_InputMap" 0 (struct))
      (set `self.Possessed Pawn` PossessedPawn))))

(event `EnhancedInput|/Game/Player/InputAction_Move`
  (params (ActionValue :type "Vector2D Structure") (ElapsedSeconds :type "Float (double-precision)") (TriggeredSeconds :type "Float (double-precision)") (InputAction :type "InputAction Object Reference" :default "/Game/Player/InputAction_Move.InputAction_Move"))
  (:`Triggered`
    (message `PlayerAction.Move` (`self.Possessed Pawn`) ActionValue)))

(event `EnhancedInput|/Game/Player/InputAction_Look`
  (params (ActionValue :type "Vector2D Structure") (ElapsedSeconds :type "Float (double-precision)") (TriggeredSeconds :type "Float (double-precision)") (InputAction :type "InputAction Object Reference" :default "/Game/Player/InputAction_Look.InputAction_Look"))
  (:`Triggered`
    (message `PlayerAction.Look` (`self.Possessed Pawn`) ActionValue)))

(event `EnhancedInput|/Game/Player/InputAction_Interact`
  (params (ActionValue :type Boolean) (ElapsedSeconds :type "Float (double-precision)") (TriggeredSeconds :type "Float (double-precision)") (InputAction :type "InputAction Object Reference" :default "/Game/Player/InputAction_Interact.InputAction_Interact"))
  (:`Started`
    (message `PlayerAction.Interact` (`self.Possessed Pawn`))))

(fn `UserConstructionScript`)